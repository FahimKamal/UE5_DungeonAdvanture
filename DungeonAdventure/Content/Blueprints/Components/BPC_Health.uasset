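; Health component that tracks its owning actor's health, defeat state and temporary invincibility.
; Health starts at max on BeginPlay, and DecreaseHealth lowers it to no less than zero, prints the result and flags defeat at zero.
; SetInvincibility uses a retriggerable delay, so repeat calls restart the window before the expiry notification fires.
; CanBeDamaged reports true only while neither defeated nor invincible; DecreaseHealth itself does not check it.
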(event Custom|SetInvincibility
  (Variables|Default|SetbIsInvincible true)
  (Utilities|FlowControl|RetriggerableDelay (Variables|Default|GetInvincibilityDuration))
  (Variables|Default|SetbIsInvincible false)
  (Default|CallInvinvibilityExpaired))

(event EventBeginPlay
  (Variables|Default|SetCurrentHealth (Variables|Default|GetMaxHealth)))

(event EventTick
  (params (DeltaSeconds :type Float%20%28single-precision%29)))

(fn DecreaseHealth
  (params (IncomingDamage :type Float%20%28double-precision%29))
  ;[0.5885 0.04236 0.06579 0.5] Decrease Health when got hit by enemy.
  (bind _output_get (Variables|Default|SetCurrentHealth (Math|Float|Max(Float) (- (Variables|Default|GetCurrentHealth) IncomingDamage) 0.0)))
  (Development|PrintText (Utilities|Text|FormatText "{actor} got hurt Health {damage}" (Utilities|GetDisplayName (Components|GetOwner)) (Utilities|String|ToString(Float) _output_get)) true true "(R=1.000000,G=0.000000,B=0.031819,A=1.000000)")
  (Variables|Default|SetIsDefeated (<= (Variables|Default|GetCurrentHealth) 0.0)))

(fn CanbeDamaged
  (return (and (not (Variables|Default|GetIsDefeated)) (not (Variables|Default|GetbIsInvincible)))))