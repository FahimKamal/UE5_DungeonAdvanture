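; Base dungeon character Blueprint shared by player and enemies, handling damage reactions.
; AnyDamage checks and reduces health through BPCHealth, then triggers knockback, an overridable HandleHitExtended hook and a brief red sprite flash.
; A timeline drives knockback by setting movement velocity away from the damage causer, scaled by strength and delta time.
; A helper toggles sprite visibility.
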(event Custom|GetKnockedBack
  (params (Attacker :type Actor%20Object%20Reference))
  ;[0.5729 0.4416 0.0959 0.5] knocked back function for player and enemy after getting hit.
  (Variables|Default|SetKnockbackDirection (Math|Vector|GetForwardVector (Math|Rotator|FindLookatRotation (Transformation|GetActorLocation Attacker) (Transformation|GetActorLocation))))
  (Components|Timeline|SetPlayRate (Variables|Default|GetKnockBackMovement) 5.0)
  (Timeline|KnockBackMovement PlayFromStart
    (:Update
      (Variables|/Script/Engine.MovementComponent|SetVelocity (Variables|Character|GetCharacterMovement) (* (Variables|Default|GetKnockbackDirection) (Variables|Default|GetKnockBackStrength) (Utilities|Time|GetWorldDeltaSeconds))))))

(event Custom|FlushSprite
  (Sprite|SetSpriteColor (Variables|Default|GetSprite) "(R=1.000000,G=0.007021,B=0.000000,A=1.000000)")
  (Utilities|FlowControl|RetriggerableDelay 0.2)
  (Sprite|SetSpriteColor (Variables|Default|GetSprite) "(R=1.000000,G=1.000000,B=1.000000,A=1.000000)"))

(event Game|Damage|EventAnyDamage
  (params (Damage :type Float%20%28single-precision%29) (DamageType :type Damage%20Type%20Object%20Reference) (InstigatedBy :type Controller%20Object%20Reference) (DamageCauser :type Actor%20Object%20Reference))
  ;[0.5885 0.04236 0.06579 0.5] Apply damage function for player and enemy.
  ;;[0.5885 0.04236 0.06579 0.5] Decrease health not getting hit my attacker for (player -> enemy) or (enemy -> player).
  (if (Default|CanbeDamaged (Variables|Default|GetBPC_Health))
    (Default|DecreaseHealth (Variables|Default|GetBPC_Health) Damage)
    (Utilities|FlowControl|Sequence
      (:then_0
        ;;[0.5729 0.4416 0.0959 0.5] Knock back on got hit. Both player and enemy.
        (CallFunction|GetKnockedBack DamageCauser))
      (:then_1
        (CallFunction|HandleHitExtended)
        (CallFunction|FlushSprite)))))

(fn ConstructionScript)

(fn SetSpriteVisibility
  (Rendering|SetVisibility (Variables|Default|GetSprite) (not (Variables|/Script/Engine.SceneComponent|GetbVisible (Variables|Default|GetSprite))) false))

(fn HandleHitExtended)